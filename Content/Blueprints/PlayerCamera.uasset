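; PlayerCamera is a player-controlled camera that pans through the level and zooms on a spring arm.
; MoveForward and MoveRight axis inputs offset the actor along its local X and Y axes by MoveSpeed, without sweep or delta-time scaling.
; Mouse wheel presses shorten or lengthen the spring arm in fixed steps, with no clamping.
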(event EventBeginPlay)

(event EventActorBeginOverlap
  (params (OtherActor :type Actor%20Object%20Reference)))

(event EventTick
  (params (DeltaSeconds :type Float%20%28single-precision%29)))

(event Input|AxisEvents|InputAxisMoveForward
  (params (AxisValue :type Float%20%28single-precision%29))
  (Transformation|AddActorLocalOffset (Math|Vector|MakeVector (* AxisValue (Variables|Default|GetMoveSpeed)) 0.0 0.0) false))

(event Input|AxisEvents|InputAxisMoveRight
  (params (AxisValue :type Float%20%28single-precision%29))
  (Transformation|AddActorLocalOffset (Math|Vector|MakeVector 0.0 (* AxisValue (Variables|Default|GetMoveSpeed)) 0.0) false))

(event Input|MouseEvents|MouseWheelUp
  (bind _springarm (Variables|Default|GetSpringArm))
  (:Pressed
    (Variables|/Script/Engine.SpringArmComponent|SetTargetArmLength _springarm (- (Variables|/Script/Engine.SpringArmComponent|GetTargetArmLength _springarm) 5e+01))))

(event Input|MouseEvents|MouseWheelDown
  (bind _springarm (Variables|Default|GetSpringArm))
  (:Pressed
    (Variables|/Script/Engine.SpringArmComponent|SetTargetArmLength _springarm (+ (Variables|/Script/Engine.SpringArmComponent|GetTargetArmLength _springarm) 5e+01))))

(fn ConstructionScript)