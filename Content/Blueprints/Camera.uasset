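; Camera Blueprint that lets the player pan and zoom the view by moving the actor itself.
; MoveForward and MoveRight axis inputs add local X and Y offsets scaled by MoveSpeed each frame, without sweep or delta-time scaling.
; Mouse wheel presses fake zoom by raising or lowering the actor along world Z by ZoomAmount, with no height limits.
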(event EventBeginPlay)

(event EventActorBeginOverlap
  (params (OtherActor :type Actor%20Object%20Reference)))

(event EventTick
  (params (DeltaSeconds :type Float%20%28single-precision%29)))

(event Input|AxisEvents|InputAxisMoveForward
  (params (AxisValue :type Float%20%28single-precision%29))
  (Transformation|AddActorLocalOffset (Math|Vector|MakeVector (* AxisValue (Variables|Default|GetMoveSpeed)) 0.0 0.0) false))

(event Input|AxisEvents|InputAxisMoveRight
  (params (AxisValue :type Float%20%28single-precision%29))
  (Transformation|AddActorLocalOffset (Math|Vector|MakeVector 0.0 (* AxisValue (Variables|Default|GetMoveSpeed)) 0.0) false))

(event Input|MouseEvents|MouseWheelDown
  (:Pressed
    (Transformation|SetActorLocation (+ (Transformation|GetActorLocation) (Math|Vector|MakeVector 0.0 0.0 (Variables|Default|GetZoomAmount))) false)))

(event Input|MouseEvents|MouseWheelUp
  (:Pressed
    (Transformation|SetActorLocation (- (Transformation|GetActorLocation) (Math|Vector|MakeVector 0.0 0.0 (Variables|Default|GetZoomAmount))) false)))

(fn ConstructionScript)